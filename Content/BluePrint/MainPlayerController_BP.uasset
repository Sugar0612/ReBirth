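; Player controller Blueprint that adds open and close animations to the pause bar handled by its parent class.
; On show, it calls the parent to open the bar, then plays the PauseWidget's PauseAnim forward.
; On hide, it plays the same animation in reverse and waits a short fixed delay before the parent closes the bar.
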(event EventBeginPlay)

(event EventTick
  (params (DeltaSeconds :type Float%20%28single-precision%29)))

(event EventShowPauseBar
  ;[1 1 1] 父类函数 实现的是打开 但是没有动画
  (|CallParentFunction)
  (bind _aspause_widget (Utilities|Casting|CastToPauseWidget (Variables|Default|GetPauseWidgetBar)))
  (UserInterface|Animation|PlayAnimation _aspause_widget (Variables|/Game/HUD/Widget/PauseWidget.PauseWidget_C|GetPauseAnim _aspause_widget) 0.0 1 "Forward" 1.0 false))

(event EventHidePauseBar
  (bind _aspause_widget (Utilities|Casting|CastToPauseWidget (Variables|Default|GetPauseWidgetBar)))
  (UserInterface|Animation|PlayAnimation _aspause_widget (Variables|/Game/HUD/Widget/PauseWidget.PauseWidget_C|GetPauseAnim _aspause_widget) 0.0 1 "Reverse" 1.0 false)
  (Utilities|FlowControl|Delay 0.25)
  ;[1 1 1] 父类函数 实现的是关闭
  (|CallParentFunction))

(fn ConstructionScript)